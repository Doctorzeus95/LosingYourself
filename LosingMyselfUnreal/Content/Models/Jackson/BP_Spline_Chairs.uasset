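; BP_Spline_Chairs is a construction-time placement actor that lays out repeated meshes, chairs by its name, along a spline.
; The construction script clears its InstancedStaticMesh component, then adds N instances at a fixed Distance interval from the spline's start.
; Each instance takes the spline's local-space location and rotation at that distance, with a hardcoded uniform scale.
; The event graph holds only disabled stubs, so nothing is scripted at runtime.
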(event EventBeginPlay)

(event Collision|EventActorBeginOverlap
  (params (OtherActor :type Actor%20Object%20Reference)))

(event EventTick
  (params (DeltaSeconds :type Float%20%28single-precision%29)))

(fn ConstructionScript
  (bind _spline (Variables|Default|GetSpline))
  (Components|InstancedStaticMesh|ClearInstances (Variables|Default|GetInstancedStaticMesh))
  (for _index (range 1 (Variables|Default|GetN))
    (Components|InstancedStaticMesh|AddInstance (Variables|Default|GetInstancedStaticMesh) (Math|Transform|MakeTransform (Spline|GetLocationatDistanceAlongSpline _spline (* (- _index 1) (Variables|Default|GetDistance)) "Local") (Spline|GetRotationatDistanceAlongSpline _spline (* (- _index 1) (Variables|Default|GetDistance)) "Local") "33.000000,33.000000,33.000000") false)))